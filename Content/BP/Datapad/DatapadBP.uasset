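; DatapadBP is a clickable datapad with Authorise and Reject sprite buttons for printing approved or rejected stickers.
; It enables click events on the player controller at BeginPlay, and each button plays a press sound and finds its sticker actor by class.
; A shared PrintingTheSicker function prints the chosen sticker with a printing sound only when both sticker actors report CanBePrinted.
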(event `self.ReceiveBeginPlay`
  (set `PlayerController.bEnableClickEvents` true (`GameplayStatics.GetPlayerController` 0)))

(event `self.Authorise_Button_Sprite.OnClicked`
  (params (TouchedComponent :type "PrimitiveComponent Object Reference") (ButtonPressed :type "Key Structure"))
  (`GameplayStatics.SpawnSound2D` "/Game/Sound/Sound_Effects/ButtonPress_Mixkit.ButtonPress_Mixkit" 1.0 1.0 0.0 null)
  (bind _returnvalue (`GameplayStatics.GetActorOfClass` "/Game/BP/Datapad/ApprovedStickersBP.ApprovedStickersBP_C"))
  (`self.PrintingTheSicker` _returnvalue))

(event `self.Reject_Button_Sprite.OnClicked`
  (params (TouchedComponent :type "PrimitiveComponent Object Reference") (ButtonPressed :type "Key Structure"))
  (`GameplayStatics.SpawnSound2D` "/Game/Sound/Sound_Effects/ButtonPress_Mixkit.ButtonPress_Mixkit" 1.0 1.0 0.0 null)
  (bind _returnvalue (`GameplayStatics.GetActorOfClass` "/Game/BP/Datapad/RejectedStickersBP.RejectedStickersBP_C"))
  (`self.PrintingTheSicker` _returnvalue))

(fn `PrintingTheSicker`
  (params (Sticker :type "/Game/BP/Datapad/AbstractSticker Object Reference"))
  (bind _returnvalue (`GameplayStatics.GetActorOfClass` "/Game/BP/Datapad/ApprovedStickersBP.ApprovedStickersBP_C"))
  (bind _returnvalue_2 (`GameplayStatics.GetActorOfClass` "/Game/BP/Datapad/RejectedStickersBP.RejectedStickersBP_C"))
  (if (and (`/Game/BP/Datapad/AbstractSticker.canBePrinted` _returnvalue) (`/Game/BP/Datapad/AbstractSticker.canBePrinted` _returnvalue_2))
    (`/Game/BP/Datapad/AbstractSticker.PrintSticker` Sticker)
    (`GameplayStatics.SpawnSound2D` "/Game/Sound/Sound_Effects/Printing_FreeSound.Printing_FreeSound" 1.0 1.0 0.0 null)))

(fn `UserConstructionScript`)