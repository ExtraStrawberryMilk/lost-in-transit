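; RejectedStickersBP is a grabbable reject sticker that slides out as if printed and sticks to parcels.
; PrintRejectedSticker enables a 1.3-second per-tick nudge along world Y, standing in for an unused Timeline.
; Collision overlaps store the BP_Parcel, even on end overlap, and Grab teleports the sticker to the mouse location.
; Tick snap-attaches it to the stored parcel whenever FirstPersonPlayer is not grabbing.
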(event `Print Rejected Sticker`
  ;[1 0.4563 0.7386] Printing
  (set `self.print` true)
  (`KismetSystemLibrary.Delay` 1.3)
  (set `self.print` false))

(event `self.Reject_Sticker Collision.OnComponentBeginOverlap`
  (params (OverlappedComponent :type "PrimitiveComponent Object Reference") (OtherActor :type "Actor Object Reference") (OtherComp :type "PrimitiveComponent Object Reference") (OtherBodyIndex :type Integer) (bFromSweep :type Boolean) (SweepResult :type "HitResult Structure (by ref)"))
  ;[0.5336 1 0.3481] Sets Parcel If Collision Occured With BP_Parcel
  (bind _asbp_parcel (cast `/Game/BP/Parcel/BP_Parcel` OtherActor))
  (set `self.Parcel` _asbp_parcel))

(event `self.Reject_Sticker Collision.OnComponentEndOverlap`
  (params (OverlappedComponent :type "PrimitiveComponent Object Reference") (OtherActor :type "Actor Object Reference") (OtherComp :type "PrimitiveComponent Object Reference") (OtherBodyIndex :type Integer))
  ;[1 0.1108 0.134] Sets Parcel If Ending Collision Occured With BP_Parcel
  (bind _asbp_parcel (cast `/Game/BP/Parcel/BP_Parcel` OtherActor))
  (set `self.Parcel` _asbp_parcel))

(event `self.ReceiveTick`
  (params (DeltaSeconds :type "Float (single-precision)"))
  (`|ExecutionSequence`
    (:`then_0`
      ;[1 0.08683 0.5803] Sticking Sticker To Parcel
      (`/Engine/EditorBlueprintResources/StandardMacros.IsValid` (`self.Parcel`)
        (:`Is Valid`
          (bind _asfirst_person_player (cast `/Game/Player/FirstPersonPlayer` (`GameplayStatics.GetPlayerCharacter` 0)))
          (if (not (`/Game/Player/FirstPersonPlayer.isGrabbing` _asfirst_person_player))
            (`self.K2_AttachToActor` (`self.Parcel`) "None" "SnapToTarget" "SnapToTarget" "SnapToTarget")
            (`KismetSystemLibrary.PrintString` "Attatched")))))
    (:`then_1`
      ;[1 0.7444 0.1372] Moving Sticker For Printing
      (if (`self.print`)
        (`self.K2_SetActorTransform` (`KismetMathLibrary.MakeTransform` (+ (`self.K2_GetActorLocation`) (0.0 0.1 0.0))))))))

(event `/Game/BP/Interfaces/Grabbable.Grab`
  (params (mouseLocation :type "Vector Structure"))
  ;[0.5477 0.8894 1] Grabbable Implementation
  (`self.K2_SetActorTransform` (`KismetMathLibrary.MakeTransform` mouseLocation) false true))

(fn `UserConstructionScript`)