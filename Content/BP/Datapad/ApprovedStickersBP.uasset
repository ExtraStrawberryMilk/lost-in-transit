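; ApprovedStickersBP is an approval sticker that tracks which parcel or bin it is touching.
; Overlap events on its authorise collision component cast the other actor to BP_Parcel, then Bin, and store the matching reference.
; Ending the overlap clears that reference, except that the parcel is kept while the sticker is flagged as Attached.
; The attaching itself and any use of the stored references are not in these graphs.
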(event `self.Authrise_Sticker_Collision.OnComponentBeginOverlap`
  (params (OverlappedComponent :type "PrimitiveComponent Object Reference") (OtherActor :type "Actor Object Reference") (OtherComp :type "PrimitiveComponent Object Reference") (OtherBodyIndex :type Integer) (bFromSweep :type Boolean) (SweepResult :type "HitResult Structure (by ref)"))
  ;[0.5336 1 0.3481] Sets Parcel If Collision Occured With BP_Parcel
  (bind _asbp_parcel (cast `/Game/BP/Parcel/BP_Parcel` OtherActor)
    (:`then`
      (set `self.Parcel` _asbp_parcel))
    (:`CastFailed`
      (bind _asbin (cast `/Game/BP/Enviroment/Bin` OtherActor))
      (set `self.Bin` _asbin))))

(event `self.Authrise_Sticker_Collision.OnComponentEndOverlap`
  (params (OverlappedComponent :type "PrimitiveComponent Object Reference") (OtherActor :type "Actor Object Reference") (OtherComp :type "PrimitiveComponent Object Reference") (OtherBodyIndex :type Integer))
  ;[1 0.1108 0.134] Sets Parcel If Ending Collision Occured With BP_Parcel
  (cast `/Game/BP/Parcel/BP_Parcel` OtherActor
    (:`then`
      (if (not (`self.Attached`))
        (set `self.Parcel` null)))
    (:`CastFailed`
      (cast `/Game/BP/Enviroment/Bin` OtherActor)
      (set `self.Bin` null))))

(fn `UserConstructionScript`)