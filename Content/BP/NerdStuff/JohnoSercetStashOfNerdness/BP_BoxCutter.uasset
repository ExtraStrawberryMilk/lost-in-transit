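; BP_BoxCutter is a grabbable box cutter that opens the parcel-top UI when released over the current parcel.
; Grab moves it to the mouse, and Box overlaps track the hovered parcel or customer.
; A fast looping timer polls for release while no WBP_TopOfParcel is open, then returns the cutter to a fixed shelf position.
; Dropping on the parcel creates that widget, while the customer only triggers a debug joke.
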(event `self.ReceiveBeginPlay`
  (`KismetSystemLibrary.K2_SetTimerDelegate` (delegate `Loop`) 0.02 true))

(event `Loop`
  (bind _foundwidgets (`WidgetBlueprintLibrary.GetAllWidgetsOfClass` "/Game/BP/NerdStuff/JohnoSercetStashOfNerdness/WBP_TopOfParcel.WBP_TopOfParcel_C"))
  (if (and (<= (`KismetArrayLibrary.Array_Length` _foundwidgets) 0) (not (`/Game/Player/FirstPersonPlayer.isGrabbing` (`/Game/BP/commonCalls.getPlayer`))))
    (`/Engine/EditorBlueprintResources/StandardMacros.IsValid` (`self.hoveringActor`)
      (:`Is Valid`
        (bind _actortype (`self.getActorType`))
        (switch `/Game/BP/NerdStuff/JohnoSercetStashOfNerdness/cutterActorTypes` _actortype
          (:`NewEnumerator0`
            (`KismetSystemLibrary.PrintString` "AHAHAHAHA OH NOOO THE CUSTOMER!!!")
            (`self.backToShelve`))
          (:`NewEnumerator1`
            (bind _returnvalue (`|CreateWidget` "/Game/BP/NerdStuff/JohnoSercetStashOfNerdness/WBP_TopOfParcel.WBP_TopOfParcel_C"))
            (`UserWidget.AddToViewport` _returnvalue 0)
            (`KismetSystemLibrary.PrintString` "THINK ABOUT THE PARCELS FEELING ;(")
            (`self.backToShelve`))
          (:`NewEnumerator2`
            (`self.backToShelve`))))
      (:`Is Not Valid`
        (`self.backToShelve`)))))

(event `/Game/BP/Interfaces/Grabbable.Grab`
  (params (mouseLocation :type "Vector Structure"))
  (`self.K2_SetActorTransform` (`KismetMathLibrary.MakeTransform` mouseLocation (struct :`Yaw` 90.0) (`self.GetActorScale3D`)) false true))

(event `self.Box.OnComponentBeginOverlap`
  (params (OverlappedComponent :type "PrimitiveComponent Object Reference") (OtherActor :type "Actor Object Reference") (OtherComp :type "PrimitiveComponent Object Reference") (OtherBodyIndex :type Integer) (bFromSweep :type Boolean) (SweepResult :type "HitResult Structure (by ref)"))
  (bind _asbp_parcel (cast `/Game/BP/Parcel/BP_Parcel` OtherActor)
    (:`then`
      (set `self.hoveringActor` _asbp_parcel))
    (:`CastFailed`
      (bind _ascustomer (cast `/Game/BP/Enviroment/Customer` OtherActor))
      (set `self.hoveringActor` _ascustomer))))

(event `self.Box.OnComponentEndOverlap`
  (params (OverlappedComponent :type "PrimitiveComponent Object Reference") (OtherActor :type "Actor Object Reference") (OtherComp :type "PrimitiveComponent Object Reference") (OtherBodyIndex :type Integer))
  (cast `/Game/BP/Parcel/BP_Parcel` OtherActor
    (:`then`
      (set `self.hoveringActor` null))
    (:`CastFailed`
      (cast `/Game/BP/Enviroment/Customer` OtherActor)
      (set `self.hoveringActor` null))))

(fn `backToShelve`
  (`self.K2_SetActorLocation` (175.0 70.0 90.0)))

(fn `getActorType`
  (returns (ActorType :type "/Game/BP/NerdStuff/JohnoSercetStashOfNerdness/cutterActorTypes Enum"))
  (if (== (`self.hoveringActor`) (`/Game/BP/commonCalls.getParcel`))
    (return "NewEnumerator1")
    (elif (== (`self.hoveringActor`) (`/Game/BP/commonCalls.getCustomer`))
      (return "NewEnumerator0")
      (else
        (return "NewEnumerator2")))))

(fn `UserConstructionScript`)