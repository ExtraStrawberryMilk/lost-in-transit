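; Sortable parcel actor that slides along Y, can be dragged no lower than the conveyor belt, and opens an information widget on interaction.
; GenerateRandomParcel rolls weight class, weight, stamp, sender and receiver, using FailChance for potentially bad weights or stamps, then caches validity.
; DeleteParcel compares the approved or rejected sticker against that validity, updates FirstPersonPlayer's sorting counters, returns the sticker to spawn and destroys the parcel.
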(event `setPhysics`
  (params (Simulate :type Boolean))
  (`PrimitiveComponent.SetSimulatePhysics` (`self.Parcel_Sprite`) Simulate))

(event `Move`
  (params (Speed :type "Float (double-precision)"))
  (bind (_returnvalue_x _returnvalue_y _returnvalue_z) (`KismetMathLibrary.BreakVector` (`self.K2_GetActorLocation`)))
  ;[0.252 0.5497 1] Moves Parcel Left or Right based on Given Speed
  (`self.K2_SetActorTransform` (`KismetMathLibrary.MakeTransform` (`KismetMathLibrary.MakeVector` _returnvalue_x (+ _returnvalue_y Speed) _returnvalue_z) (struct :`Yaw` 90.0) (`self.GetActorScale3D`)) false true))

(event `/Game/BP/Interfaces/Interactable.Interact`
  (bind _asfirst_person_player (cast `/Game/Player/FirstPersonPlayer` (`GameplayStatics.GetPlayerPawn` 0)))
  (set `/Game/Player/FirstPersonPlayer.notPaused` false _asfirst_person_player)
  (bind _foundwidgets (`WidgetBlueprintLibrary.GetAllWidgetsOfClass` "/Game/BP/UI/WBP_ParcelInfomation.WBP_ParcelInfomation_C"))
  (`/Engine/EditorBlueprintResources/StandardMacros.IsValid` (`|GetArrayItem` _foundwidgets)
    (:`Is Not Valid`
      (bind _foundwidgets_2 (`WidgetBlueprintLibrary.GetAllWidgetsOfClass` "/Game/BP/UI/Requirements.Requirements_C"))
      (bind _output (`|GetArrayItem` _foundwidgets_2))
      (`/Engine/EditorBlueprintResources/StandardMacros.IsValid` _output
        (:`Is Valid`
          (`Widget.RemoveFromParent` _output))
        (:`Is Not Valid`
          _))
      (bind _returnvalue (`|CreateWidget` "/Game/BP/UI/WBP_ParcelInfomation.WBP_ParcelInfomation_C"))
      (`UserWidget.AddToViewport` _returnvalue 0))))

(event `self.ReceiveBeginPlay`
  ;[1 0.4516 0.8324] Creates Parcel Weight Widget
  (bind _returnvalue (`|CreateWidget` "/Game/BP/UI/ParcelWeight.ParcelWeight_C"))
  (`UserWidget.AddToViewport` _returnvalue 0))

(event `GenerateRandomParcel`
  (`self.setRandomWeightClass`)
  (`self.setWeightRandom`)
  (`self.setRandomStamp`)
  (bind (_name _address) (`self.createNameAndAddress`))
  (set `self.senderName` _name)
  (set `self.senderAddress` _address)
  (bind (_name_2 _address_2) (`self.createNameAndAddress`))
  (set `self.receiverName` _name_2)
  (set `self.receiverAddress` _address_2)
  (`self.isParcelValid`))

(event `/Game/BP/Interfaces/Grabbable.Grab`
  (params (mouseLocation :type "Vector Structure"))
  (bind _returnvalue (+ mouseLocation_Z -25.0))
  (bind _returnvalue_2 (`GameplayStatics.GetActorOfClass` "/Game/BP/Enviroment/BP_ConveyorBelt.BP_ConveyorBelt_C"))
  (bind (_returnvalue_x _returnvalue_y _returnvalue_z) (`KismetMathLibrary.BreakVector` (`self.K2_GetActorLocation` _returnvalue_2)))
  (`self.K2_SetActorTransform` (`KismetMathLibrary.MakeTransform` (`KismetMathLibrary.MakeVector` mouseLocation_X mouseLocation_Y (select `bool` (< _returnvalue _returnvalue_z) :`false` _returnvalue :`true` _returnvalue_z)) (struct :`Yaw` 90.0) (`self.GetActorScale3D`)) false true)
  (set `self.lastPosition` (`KismetMathLibrary.MakeVector` mouseLocation_X mouseLocation_Y mouseLocation_Z)))

(fn `createNameAndAddress`
  (returns (Name :type String) (Address :type String))
  (locals (FailChance :type Integer :default 15) (FirstNames :type "Array of String") (LastNames :type "Array of String") (StreetPrefix :type "Array of String") (StreetSuffix :type "Array of String"))
  (return (select `bool` (<= 0 (`KismetMathLibrary.RandomIntegerInRange` 0 100)) :`true` (`KismetStringLibrary.Concat_StrStr` (`KismetArrayLibrary.Array_Random` (`local.FirstNames`)) " " (`KismetArrayLibrary.Array_Random` (`local.LastNames`)))) (select `bool` (<= 0 (`KismetMathLibrary.RandomIntegerInRange` 0 100)) :`true` (`KismetStringLibrary.Concat_StrStr` (`KismetStringLibrary.Conv_IntToString` (`KismetMathLibrary.RandomIntegerInRange` 100 200)) " " (`KismetArrayLibrary.Array_Random` (`local.StreetPrefix`)) " " (`KismetArrayLibrary.Array_Random` (`local.StreetSuffix`))))))

(fn `deleteParcel`
  (locals (pareclValue :type String) (player :type "/Game/Player/FirstPersonPlayer Object Reference"))
  (bind _player (`local.player`))
  (bind _player_2 (`local.player`))
  ;[0.4976 0.4781 1] Increases The Number Of Sorted Parcels by 1
  (bind _asfirst_person_player (cast `/Game/Player/FirstPersonPlayer` (`GameplayStatics.GetPlayerCharacter` 0)))
  (bind _output_get (set `local.player` _asfirst_person_player))
  (set `/Game/Player/FirstPersonPlayer.NumberParcelsSorted` (+ (`/Game/Player/FirstPersonPlayer.NumberParcelsSorted` (`local.player`)) 1.0) _output_get)
  ;[0.9696 1 0.2359] Branches Logic Depending If The Parcel Is Correctly Sorted Or Not
  (bind _result (`self.isParcelCorrectlySorted`))
  (switch `string` (`KismetMathLibrary.SelectString` "Correct" "Incorrect" _result)
    (:`Correct`
      ;[1 0.6217 0.4253] Adds 1 To Correctly / Incorrectly Sorted Parcels And Sents The Sticker Behind The Datapad Then Destroys The Parcel
      (set `/Game/Player/FirstPersonPlayer.ParcelsSortedCorrectly` (+ (`/Game/Player/FirstPersonPlayer.ParcelsSortedCorrectly` _player_2) 1.0) _player_2))
    (:`Incorrect`
      (set `/Game/Player/FirstPersonPlayer.ParcelsSortedIncorrectly` (+ (`/Game/Player/FirstPersonPlayer.ParcelsSortedIncorrectly` _player) 1.0) _player)))
  (`/Game/BP/Datapad/AbstractSticker.backToSpawn` (`self.sticker`))
  (`self.K2_DestroyActor`))

(fn `isOnScreen`
  (returns (result :type Boolean))
  (bind (_returnvalue_x _returnvalue_y) (`KismetMathLibrary.BreakVector2D` (`WidgetLayoutLibrary.GetViewportSize`)))
  (bind _screenlocation (`PlayerController.ProjectWorldLocationToScreen` (`GameplayStatics.GetPlayerController` 0) (`self.K2_GetActorLocation`) true))
  (return (and (> (`KismetMathLibrary.BreakVector2D` _screenlocation) 0.0) (> (`.Y` (`KismetMathLibrary.BreakVector2D` _screenlocation)) 0.0) (< (`KismetMathLibrary.BreakVector2D` _screenlocation) _returnvalue_x) (< (`.Y` (`KismetMathLibrary.BreakVector2D` _screenlocation)) _returnvalue_y))))

(fn `isParcelCorrectlySorted`
  (returns (Result :type Boolean))
  (bind _isvalid (`self.isValid`))
  ;[0.4824 1 0.05777] Returns True If RejectSticker is on a InValid Parcel or an Approved Sticker is on a Valid Parcel
  (bind _outactors (`GameplayStatics.GetAllActorsOfClass` "/Game/BP/Datapad/ApprovedStickersBP.ApprovedStickersBP_C"))
  (bind _outactors_2 (`GameplayStatics.GetAllActorsOfClass` "/Game/BP/Datapad/RejectedStickersBP.RejectedStickersBP_C"))
  (return (or (and (== (`self.sticker`) (`|GetArrayItem` _outactors_2)) (not _isvalid)) (and _isvalid (== (`|GetArrayItem` _outactors) (`self.sticker`))))))

(fn `isParcelValid`
  (returns (result :type Boolean))
  (bind (_x _y) (`KismetMathLibrary.BreakVector2D` (`BlueprintMapLibrary.Map_Find` (`self.weightClassToWeight`) (`self.weightClass`))))
  (bind _output_get (set `self.isValid` (and (`KismetMathLibrary.InRange_FloatFloat` (`self.weight`) _x _y) (!= (`KismetArrayLibrary.Array_Find` (`self.validStamps`) (`self.stamp`)) -1) (not (or (`KismetStringLibrary.EqualEqual_StrStr` (`self.senderName`)) (`KismetStringLibrary.EqualEqual_StrStr` (`self.receiverName`)) (`KismetStringLibrary.EqualEqual_StrStr` (`self.senderAddress`)) (`KismetStringLibrary.EqualEqual_StrStr` (`self.receiverAddress`)))))))
  (return _output_get))

(fn `setRandomStamp`
  (locals (FailChance :type Integer :default 35))
  ;[0.9679 0.621 1] Either Gets a Random Stamp From Valid Stamps [Set In The Level] or Gets a Random Stamp From All The Stamps [Set In gameInstance]
  (if (<= (`KismetMathLibrary.RandomIntegerInRange` 0 100) (`local.FailChance`))
    (bind _asgame_instance (cast `/Game/Player/gameInstance` (`GameplayStatics.GetGameInstance`)))
    (bind _keys (`BlueprintMapLibrary.Map_Keys` (`/Game/Player/gameInstance.allStamps` _asgame_instance)))
    (set `self.stamp` (`|GetArrayItem` _keys (`KismetMathLibrary.RandomIntegerInRange` 0 (- (`KismetArrayLibrary.Array_Length` _keys) 1))))
    (else
      (set `self.stamp` (`|GetArrayItem` (`self.validStamps`) (`KismetMathLibrary.RandomIntegerInRange` 0 5))))))

(fn `setRandomWeightClass`
  (switch `int` (`KismetMathLibrary.RandomIntegerInRange` 0 2)
    (:`0`
      (set `self.weightClass` "A"))
    (:`1`
      (set `self.weightClass` "B"))
    (:`2`
      (set `self.weightClass` "C"))))

(fn `setWeightRandom`
  (locals (FailChance :type Integer :default 30))
  (bind (_x _y) (`KismetMathLibrary.BreakVector2D` (`BlueprintMapLibrary.Map_Find` (`self.weightClassToWeight`) (`self.weightClass`))))
  (bind _returnvalue (`KismetMathLibrary.RandomFloatInRange` _x _y))
  ;[0.9005 0.3262 1] Converts the Random Weight Into a 2dp Weight (3.238123 -> 3.23)
  (set `self.weight` (/ (`KismetMathLibrary.Conv_IntToDouble` (`KismetMathLibrary.FFloor` (* (select `bool` (<= (`local.FailChance`) (`KismetMathLibrary.RandomIntegerInRange` 0 100)) :`false` (+ _returnvalue (/ (+ _x _y) 2.0)) :`true` _returnvalue) 100.0))) 100.0)))

(fn `UserConstructionScript`)