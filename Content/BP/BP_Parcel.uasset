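; Parcel actor that assigns itself a random sender and receiver from the Customers data table when it spawns.
; Each pick converts a random integer from 1 to the row count into a row name, so it relies on sequentially numbered rows.
; BeginPlay rerolls both until they differ in name or address, then prints a creation message.
; DeleteParcel destroys the actor.
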(event `self.ReceiveBeginPlay`
  (`self.setRandomSender` :!label _label)
  (`self.setRandomReceiver`)
  (`self.isPeopleEqual`)
  (if (`self.isPeopleSame`)
    (goto _label)
    (else
      (`KismetSystemLibrary.PrintString` "Created Parcel"))))

(fn `deleteParcel`
  (`self.K2_DestroyActor`))

(fn `isPeopleEqual`
  (bind (_name _address) (break `/Game/Structures/F_Customer` (`self.sender`)))
  (bind (_name_2 _address_2) (break `/Game/Structures/F_Customer` (`self.receiver`)))
  (if (and (== _name _name_2) (== _address _address_2))
    (set `self.isPeopleSame` true)
    (else
      (set `self.isPeopleSame` false))))

(fn `setRandomReceiver`
  (bind _outrownames (`DataTableFunctionLibrary.GetDataTableRowNames` "/Game/Structures/Customers.Customers"))
  (bind _returnvalue (`|GetDataTableRow` "/Game/Structures/Customers.Customers" (`KismetStringLibrary.Conv_StringToName` (`KismetStringLibrary.Conv_IntToString` (`KismetMathLibrary.RandomIntegerInRange` 1 (`KismetArrayLibrary.Array_Length` _outrownames)))))
    (:`then`
      (set `self.receiver` _returnvalue))))

(fn `setRandomSender`
  (bind _outrownames (`DataTableFunctionLibrary.GetDataTableRowNames` "/Game/Structures/Customers.Customers"))
  (bind _returnvalue (`|GetDataTableRow` "/Game/Structures/Customers.Customers" (`KismetStringLibrary.Conv_StringToName` (`KismetStringLibrary.Conv_IntToString` (`KismetMathLibrary.RandomIntegerInRange` 1 (`KismetArrayLibrary.Array_Length` _outrownames)))))
    (:`then`
      (set `self.sender` _returnvalue))))

(fn `UserConstructionScript`)