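; BP_NamesNote2 is a draggable paper note that opens the WBP_NamesNote widget on interaction.
; Grab follows the mouse, clamped above the conveyor belt; Yeat restores physics and can fling the sprite along Y.
; Overlapping a Bench flattens it and disables physics, while Slide_List makes Tick slide it briefly.
; Helpers set valid date, parcel weight class and image, or pick a different random weight class.
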(event `self.Grab`
  (params (mouseLocation :type "Vector Structure"))
  (if (not (`self.Slide`))
    (bind _returnvalue (`GameplayStatics.GetActorOfClass` "/Game/BP/Enviroment/BP_ConveyorBelt.BP_ConveyorBelt_C"))
    (bind (_returnvalue_x _returnvalue_y _returnvalue_z) (`KismetMathLibrary.BreakVector` (`self.K2_GetActorLocation` _returnvalue)))
    (bind _returnvalue_2 (select `bool` (< (+ mouseLocation_Z -2.0) _returnvalue_z) :`false` mouseLocation_Z :`true` (+ _returnvalue_z 2.0)))
    (`self.K2_SetActorTransform` (`KismetMathLibrary.MakeTransform` (`KismetMathLibrary.MakeVector` mouseLocation_X mouseLocation_Y _returnvalue_2) (struct :`Pitch` 90.0 :`Yaw` 90.0) (`self.GetActorScale3D`)) false true)
    (set `self.lastPos` (`KismetMathLibrary.MakeVector` mouseLocation_X mouseLocation_Y _returnvalue_2))))

(event `self.Box.OnComponentBeginOverlap`
  (params (OverlappedComponent :type "PrimitiveComponent Object Reference") (OtherActor :type "Actor Object Reference") (OtherComp :type "PrimitiveComponent Object Reference") (OtherBodyIndex :type Integer) (bFromSweep :type Boolean) (SweepResult :type "HitResult Structure (by ref)"))
  (bind _papersprite (`self.PaperSprite`))
  (bind (_relativelocation_x _relativelocation_y) (`KismetMathLibrary.BreakVector` (`SceneComponent.RelativeLocation` _papersprite)))
  (cast `/Game/BP/Enviroment/Bench` OtherActor)
  (`SceneComponent.K2_SetWorldRotation` _papersprite (struct :`Pitch` 90.0 :`Yaw` 90.0) false true)
  (`SceneComponent.K2_SetRelativeLocation` _papersprite (`KismetMathLibrary.MakeVector` _relativelocation_x _relativelocation_y 86.0) false false)
  (`self.K2_SetActorRotation` (struct :`Pitch` 10.0 :`Roll` 90.0))
  (`self.setPhysics` false))

(event `/Game/BP/Interfaces/Interactable.Interact`
  (bind _foundwidgets (`WidgetBlueprintLibrary.GetAllWidgetsOfClass` "/Game/BP/UI/WBP_NamesNote.WBP_NamesNote_C"))
  (`/Engine/EditorBlueprintResources/StandardMacros.IsValid` (`|GetArrayItem` _foundwidgets)
    (:`Is Not Valid`
      (bind _returnvalue (`|CreateWidget` "/Game/BP/UI/WBP_NamesNote.WBP_NamesNote_C"))
      (`UserWidget.AddToViewport` _returnvalue 0))))

(event `Slide_List`
  ;[1 1 1] Time to slide
  (set `self.Slide` true)
  (`self.setPhysics` false)
  (`KismetSystemLibrary.Delay` 2.0)
  (set `self.Slide` false))

(event `self.ReceiveTick`
  (params (DeltaSeconds :type "Float (single-precision)"))
  ;[1 1 1] Slide Distance
  (if (`self.Slide`)
    (`self.K2_SetActorTransform` (`KismetMathLibrary.MakeTransform` (+ (`self.K2_GetActorLocation`) (0.0 -0.05 -0.175)) (struct :`Pitch` 90.0 :`Yaw` 90.0) (`self.GetActorScale3D`)))
    (`self.K2_SetActorRotation` (struct :`Pitch` 10.0 :`Roll` 90.0))))

(event `/Game/BP/Interfaces/Yeatable.setPhysicss`
  (params (Sim :type Boolean))
  (`self.setPhysics` Sim))

(event `/Game/BP/Interfaces/Yeatable.Yeat`
  (params (mousePos :type "Vector Structure"))
  (bind (_returnvalue_x _returnvalue_y) (`KismetMathLibrary.BreakVector` (- mousePos (`self.lastPos`))))
  (`self.setPhysics` true)
  (if (not (`/Game/Player/FirstPersonPlayer.canInteract` (`/Game/BP/commonCalls.getPlayer`)))
    (`PrimitiveComponent.AddImpulse` (`self.PaperSprite`) (`KismetMathLibrary.MakeVector` 0.0 (* _returnvalue_y 3.0)) "None" false)))

(fn `randomNot`
  (params (`not this` :type String))
  (returns (random :type String))
  (locals (NewLocalVar :type "Array of String"))
  (bind _output_get (set `local.NewLocalVar` (`self.WeightClassArray`)))
  (`KismetArrayLibrary.Array_RemoveItem` _output_get `not this`)
  (return (`KismetArrayLibrary.Array_Random` _output_get)))

(fn `Set_Valid_Date`
  (set `self.Date` (`/Game/Player/gameInstance.Day` (`/Game/BP/commonCalls.getGameInstance`))))

(fn `Set_Valid_Image`
  (set `self.Image` true))

(fn `Set_Valid_weight_Class`
  (bind _outactors (`GameplayStatics.GetAllActorsOfClass` "/Game/BP/Parcel/BP_Parcel.BP_Parcel_C"))
  (set `self.Weight Class` (`/Game/BP/Parcel/BP_Parcel.weightClass` (`|GetArrayItem` _outactors))))

(fn `setPhysics`
  (params (Simulate :type Boolean))
  (`PrimitiveComponent.SetSimulatePhysics` (`self.PaperSprite`) Simulate))

(fn `UserConstructionScript`)