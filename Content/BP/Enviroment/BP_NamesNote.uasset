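; Paper note actor for a list of names that can be read, dragged with the mouse and slid along.
; Interact adds the WBP_NamesNote widget to the viewport unless one is already open.
; Slide_List raises a flag for a tenth of a second, during which Tick nudges the note along negative X.
; Grab follows the mouse when not sliding, keeps Z above BP_ConveyorBelt and stores the last position.
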(event `/Game/BP/Interfaces/Interactable.Interact`
  (bind _foundwidgets (`WidgetBlueprintLibrary.GetAllWidgetsOfClass` "/Game/BP/UI/WBP_NamesNote.WBP_NamesNote_C"))
  (`/Engine/EditorBlueprintResources/StandardMacros.IsValid` (`|GetArrayItem` _foundwidgets)
    (:`Is Not Valid`
      (bind _returnvalue (`|CreateWidget` "/Game/BP/UI/WBP_NamesNote.WBP_NamesNote_C"))
      (`UserWidget.AddToViewport` _returnvalue 0))))

(event `Slide_List`
  ;[1 1 1] Time to slide
  (set `self.Slide` true)
  (`KismetSystemLibrary.Delay` 0.1)
  (set `self.Slide` false))

(event `self.ReceiveTick`
  (params (DeltaSeconds :type "Float (single-precision)"))
  ;[1 1 1] Slide Distance
  (if (`self.Slide`)
    (`self.K2_SetActorTransform` (`KismetMathLibrary.MakeTransform` (+ (`self.K2_GetActorLocation`) (-0.5 0.0 0.0))))))

(event `/Game/BP/Interfaces/Grabbable.Grab`
  (params (mouseLocation :type "Vector Structure"))
  (if (not (`self.Slide`))
    (bind _returnvalue (`GameplayStatics.GetActorOfClass` "/Game/BP/Enviroment/BP_ConveyorBelt.BP_ConveyorBelt_C"))
    (bind (_returnvalue_x _returnvalue_y _returnvalue_z) (`KismetMathLibrary.BreakVector` (`self.K2_GetActorLocation` _returnvalue)))
    (bind _returnvalue_2 (select `bool` (< (+ mouseLocation_Z -2.0) _returnvalue_z) :`false` mouseLocation_Z :`true` (+ _returnvalue_z 2.0)))
    (`self.K2_SetActorTransform` (`KismetMathLibrary.MakeTransform` (`KismetMathLibrary.MakeVector` mouseLocation_X mouseLocation_Y _returnvalue_2) (struct) (`self.GetActorScale3D`)))
    (set `self.Las_Pos` (`KismetMathLibrary.MakeVector` mouseLocation_X mouseLocation_Y _returnvalue_2))))

(fn `NewFunction`)

(fn `Set_Physics`
  (params (NewParam :type Boolean))
  (`PrimitiveComponent.SetSimulatePhysics` (`self.PaperSprite`) NewParam))

(fn `UserConstructionScript`)