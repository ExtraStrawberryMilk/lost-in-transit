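; Permit actor that generates a customer document on spawn and opens it in a Permit widget on interaction, clearing the player's NotPaused flag.
; BeginPlay fills date, weight class and image from the current day and first BP_Parcel, then, as wired, always randomly falsifies one of them.
; Slide_ enables a one-second, per-tick movement along negative X.
; Grab is empty, and the customer's PermitIsValid lookup is unused.
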(event `self.ReceiveBeginPlay`
  ;[1 1 1] Generates Permit Infomation When Spawned In
  (`self.Set_Valid_Date`)
  (`self.Set_Valid_Date`)
  (`self.Set_Valid_weight_Class`)
  (`self.Set_Valid_Image`)
  (if (not false)
    (switch `int` (`KismetMathLibrary.RandomIntegerInRange` 1 3)
      (:`1`
        (set `self.Date` (`KismetMathLibrary.RandomIntegerInRange` 1 (- (`/Game/Player/gameInstance.Day` (`/Game/BP/commonCalls.getGameInstance`)) 1))))
      (:`2`
        (set `self.Image` false))
      (:`3`
        (bind _outactors (`GameplayStatics.GetAllActorsOfClass` "/Game/BP/Parcel/BP_Parcel.BP_Parcel_C"))
        (set `self.Weight Class` (`self.randomNot` (`/Game/BP/Parcel/BP_Parcel.weightClass` (`|GetArrayItem` _outactors))))))))

(event `Slide_`
  ;[1 1 1] Time to slide
  (set `self.Slide` true)
  (`KismetSystemLibrary.Delay` 1.0)
  (set `self.Slide` false))

(event `self.ReceiveTick`
  (params (DeltaSeconds :type "Float (single-precision)"))
  ;[1 1 1] Slide Distance
  (if (`self.Slide`)
    (`self.K2_SetActorTransform` (`KismetMathLibrary.MakeTransform` (+ (`self.K2_GetActorLocation`) (-0.5 0.0 0.0)) (struct :`Yaw` 90.0 :`Roll` -80.0) (`self.Permit Scale`)))))

(event `/Game/BP/Interfaces/Interactable.Interact`
  (bind _asfirst_person_player (cast `/Game/Player/FirstPersonPlayer` (`GameplayStatics.GetPlayerPawn` 0)))
  (set `/Game/Player/FirstPersonPlayer.notPaused` false _asfirst_person_player)
  (bind _returnvalue (`|CreateWidget` "/Game/BP/UI/Information_Widgets/Permit.Permit_C"))
  (`UserWidget.AddToViewport` _returnvalue 0))

(event `/Game/BP/Interfaces/Grabbable.Grab`
  (params (mouseLocation :type "Vector Structure")))

(fn `randomNot`
  (params (`not this` :type String))
  (returns (random :type String))
  (locals (NewLocalVar :type "Array of String"))
  (bind _output_get (set `local.NewLocalVar` (`self.WeightClassArray`)))
  (`KismetArrayLibrary.Array_RemoveItem` _output_get `not this`)
  (return (`KismetArrayLibrary.Array_Random` _output_get)))

(fn `Set_Valid_Date`
  (set `self.Date` (`/Game/Player/gameInstance.Day` (`/Game/BP/commonCalls.getGameInstance`))))

(fn `Set_Valid_Image`
  (set `self.Image` true))

(fn `Set_Valid_weight_Class`
  (bind _outactors (`GameplayStatics.GetAllActorsOfClass` "/Game/BP/Parcel/BP_Parcel.BP_Parcel_C"))
  (set `self.Weight Class` (`/Game/BP/Parcel/BP_Parcel.weightClass` (`|GetArrayItem` _outactors))))

(fn `UserConstructionScript`)