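; Conveyor belt that carries a customer's dropped parcel, with direction depending on whether it has a sticker.
; Box overlap tracks a single parcel once the customer has dropped it and clears it on exit.
; Tick sends that parcel a move message, reversing direction and increasing magnitude when no sticker exists.
; With a parcel tracked, the DeleteHitBox overlap sends the customer away for removal and deletes the parcel.
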(event `self.ReceiveTick`
  (params (DeltaSeconds :type "Float (single-precision)"))
  (bind _actor (`self.Actor`))
  (`/Engine/EditorBlueprintResources/StandardMacros.IsValid` _actor
    (:`Is Valid`
      (bind _asbp_parcel (cast `/Game/BP/Parcel/BP_Parcel` _actor))
      (`/Engine/EditorBlueprintResources/StandardMacros.IsValid` (`/Game/BP/Parcel/BP_Parcel.sticker` _asbp_parcel)
        (:`Is Valid`
          (message `/Game/BP/Interfaces/Grabbable.MoveOnConveyor` _asbp_parcel 1.0))
        (:`Is Not Valid`
          (message `/Game/BP/Interfaces/Grabbable.MoveOnConveyor` _asbp_parcel -3.0))))))

(event `self.Box.OnComponentBeginOverlap`
  (params (OverlappedComponent :type "PrimitiveComponent Object Reference") (OtherActor :type "Actor Object Reference") (OtherComp :type "PrimitiveComponent Object Reference") (OtherBodyIndex :type Integer) (bFromSweep :type Boolean) (SweepResult :type "HitResult Structure (by ref)"))
  (bind _customer (`/Game/BP/commonCalls.getCustomer`))
  ;[0 0.7347 1] Sets Parcel if parcel overlaps conveyor belt
  (bind _asbp_parcel (cast `/Game/BP/Parcel/BP_Parcel` OtherActor))
  (`/Engine/EditorBlueprintResources/StandardMacros.IsValid` _customer
    (:`Is Valid`
      (if (`/Game/BP/Enviroment/Customer.Parcel Dropped` _customer)
        (set `self.Actor` _asbp_parcel)))))

(event `self.Box.OnComponentEndOverlap`
  (params (OverlappedComponent :type "PrimitiveComponent Object Reference") (OtherActor :type "Actor Object Reference") (OtherComp :type "PrimitiveComponent Object Reference") (OtherBodyIndex :type Integer))
  ;[1 0 0] Sets Parcel to null if moved off conveyor belt
  (cast `/Game/BP/Parcel/BP_Parcel` OtherActor)
  (set `self.Actor` null))

(event `self.deleteHitBox.OnComponentBeginOverlap`
  (params (OverlappedComponent :type "PrimitiveComponent Object Reference") (OtherActor :type "Actor Object Reference") (OtherComp :type "PrimitiveComponent Object Reference") (OtherBodyIndex :type Integer) (bFromSweep :type Boolean) (SweepResult :type "HitResult Structure (by ref)"))
  (cast `/Game/BP/Parcel/BP_Parcel` OtherActor)
  (`/Engine/EditorBlueprintResources/StandardMacros.IsValid` (`self.Actor`)
    (:`Is Valid`
      (bind _returnvalue (`GameplayStatics.GetActorOfClass` "/Game/BP/Enviroment/Customer.Customer_C"))
      (`/Engine/EditorBlueprintResources/StandardMacros.IsValid` _returnvalue
        (:`Is Valid`
          (`/Game/BP/Enviroment/Customer.moveTo` _returnvalue 3.0 0.45 true)
          (`/Game/BP/Parcel/BP_Parcel.deleteParcel` (`/Game/BP/commonCalls.getParcel`)))))))

(fn `UserConstructionScript`)