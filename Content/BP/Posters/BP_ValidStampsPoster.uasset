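; Interactable poster actor that opens a UI showing the level's valid stamps.
; On Interact, it does nothing if its poster widget is already open; otherwise it closes any open weight class poster.
; It then creates the valid stamps widget with the LevelManager's ValidStamps, plays an opening sound and adds it to the viewport.
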(event `/Game/BP/Interfaces/Interactable.Interact`
  (bind _foundwidgets (`WidgetBlueprintLibrary.GetAllWidgetsOfClass` "/Game/BP/UI/Information_Widgets/WBP_ValidStampsPoster.WBP_ValidStampsPoster_C"))
  (`/Engine/EditorBlueprintResources/StandardMacros.IsValid` (`|GetArrayItem` _foundwidgets)
    (:`Is Not Valid`
      (bind _foundwidgets_2 (`WidgetBlueprintLibrary.GetAllWidgetsOfClass` "/Game/BP/UI/Information_Widgets/WBP_WeightClassPoster.WBP_WeightClassPoster_C"))
      (bind _output (`|GetArrayItem` _foundwidgets_2))
      (`/Engine/EditorBlueprintResources/StandardMacros.IsValid` _output
        (:`Is Valid`
          (`Widget.RemoveFromParent` _output))
        (:`Is Not Valid`
          _))
      (bind _returnvalue (`GameplayStatics.GetActorOfClass` "/Game/BP/LevelManager.LevelManager_C"))
      (bind _returnvalue_2 (`|CreateWidget` "/Game/BP/UI/Information_Widgets/WBP_ValidStampsPoster.WBP_ValidStampsPoster_C" null (`/Game/BP/LevelManager.validStamps` _returnvalue)))
      (`GameplayStatics.SpawnSound2D` "/Game/Sound/Sound_Effects/OpenPoster_Mixkit.OpenPoster_Mixkit" 1.0 1.0 0.0 null)
      (`UserWidget.AddToViewport` _returnvalue_2 0))))

(fn `UserConstructionScript`)